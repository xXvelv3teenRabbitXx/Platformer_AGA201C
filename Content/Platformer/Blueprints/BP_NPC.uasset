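; BP_NPC is a platformer NPC that shows an interaction prompt and plays timed dialogue through the player.
; Its trigger zone toggles the prompt when an actor tagged Player enters or leaves.
; Reset_Dialogue, which is not called within this graph, restarts the sequence from the first line.
; Update_Dialogue writes each line to the cached third-person character's CurrentDialogueText, re-triggers itself after a fixed delay, then clears the text.
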(event `self.NPC_Trigger_Zone.OnComponentBeginOverlap`
  (params (OverlappedComponent :type "PrimitiveComponent Object Reference") (OtherActor :type "Actor Object Reference") (OtherComp :type "PrimitiveComponent Object Reference") (OtherBodyIndex :type Integer) (bFromSweep :type Boolean) (SweepResult :type "HitResult Structure (by ref)"))
  ;[0.7608 0 0] Widget_Visibility
  ;;[0.7608 0.2902 0.2902] Begin_Overlap
  (if (`self.ActorHasTag` OtherActor "Player")
    (`SceneComponent.SetVisibility` (`self.Interaction_Prompt`) true false)))

(event `self.NPC_Trigger_Zone.OnComponentEndOverlap`
  (params (OverlappedComponent :type "PrimitiveComponent Object Reference") (OtherActor :type "Actor Object Reference") (OtherComp :type "PrimitiveComponent Object Reference") (OtherBodyIndex :type Integer))
  ;[0.7608 0 0] Widget_Visibility
  ;;[0.7608 0.2902 0.2902] End_Overlap
  (if (`self.ActorHasTag` OtherActor "Player")
    (`SceneComponent.SetVisibility` (`self.Interaction_Prompt`) false false)))

(event `self.ReceiveBeginPlay`
  ;[0.1294 0.4157 1] Get_Player_Reference
  (bind _asbp_third_person_character (cast `/Game/Platformer/Blueprints/BP_ThirdPersonCharacter` (`GameplayStatics.GetPlayerPawn` 0)))
  (set `self.Player_Reference` _asbp_third_person_character))

(event `Update_Dialogue`
  ;[1 0.3216 0.8039] NPC_Dialogue
  ;;[1 0.3216 0.8039] Update_Dialogue
  (set `/Game/Platformer/Blueprints/BP_ThirdPersonCharacter.Current_Dialogue_Text` (`|GetArrayItem` (`self.Dialogue_Lines`) (`self.Current_Diaglogue_Line`)) (`self.Player_Reference`))
  (set `self.Current_Diaglogue_Line` (+ (`self.Current_Diaglogue_Line`) 1))
  (`KismetSystemLibrary.Delay` 2.0)
  (if (!= (`self.Current_Diaglogue_Line`) (`KismetArrayLibrary.Array_Length` (`self.Dialogue_Lines`)))
    ;;[1 0.3216 0.8039] Cycle_Dialogue
    (`self.Update_Dialogue`)
    (else
      ;;[1 0.3216 0.8039] Stop_Dialogue
      (set `/Game/Platformer/Blueprints/BP_ThirdPersonCharacter.Current_Dialogue_Text` "" (`self.Player_Reference`)))))

(event `Reset_Dialogue`
  ;[1 0.3216 0.8039] NPC_Dialogue
  ;;[1 0.3216 0.8039] Reset_Dialogue
  (set `self.Current_Diaglogue_Line` 0)
  (`self.Update_Dialogue`))

(fn `UserConstructionScript`)