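; BP_Platform_Moving is a platformer platform that shuttles back and forth along a Direction vector.
; BeginPlay enables movement and starts a looping timer that negates Direction every MovementDuration seconds.
; Each Tick offsets the actor by the normalized Direction times Speed without sweeping.
; The step is not scaled by delta time, so travel speed and distance depend on frame rate.
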(event `self.ReceiveBeginPlay`
  ;[0.003922 0.6157 0] Platform Flip Direction
  (`|ExecutionSequence`
    (:`then_0`
      (set `self.Can_Platform_Move` true))
    (:`then_1`
      (`KismetSystemLibrary.K2_SetTimerDelegate` (delegate `Flip_Direction`) (`self.Movement_Duration`) true))))

(event `Flip_Direction`
  ;[0.003922 0.6157 0] Platform Flip Direction
  (set `self.Direction` (* (`self.Direction`) -1.0)))

(event `self.ReceiveTick`
  (params (DeltaSeconds :type "Float (single-precision)"))
  ;[1 0.4941 0] Platform Movement
  (if (`self.Can_Platform_Move`)
    (`self.K2_AddActorWorldOffset` (* (`KismetMathLibrary.Normal` (`self.Direction`)) (`self.Speed`)))))

(fn `UserConstructionScript`)