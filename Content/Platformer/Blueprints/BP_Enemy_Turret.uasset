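; Enemy turret Blueprint that fires BP_Bullet actors from its FiringPoint on a repeating timer.
; On BeginPlay, UseScattershot selects single shots or bursts with random yaw spread, and each firing event re-calls itself after a FiringDelay.
; When LookAtPlayer is set, Tick turns SMStem toward the player pawn using only X and Y, applying the look-at result as relative rotation.
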(event `self.ReceiveTick`
  (params (DeltaSeconds :type "Float (single-precision)"))
  (bind (_returnvalue_x _returnvalue_y) (`KismetMathLibrary.BreakVector` (`self.K2_GetActorLocation`)))
  (bind (_returnvalue_x_2 _returnvalue_y_2) (`KismetMathLibrary.BreakVector` (`self.K2_GetActorLocation` (`GameplayStatics.GetPlayerPawn` 0))))
  ;[1 0.4941 0] Rotate_Turret_to_Look_At_Player
  (if (`self.Look_At_Player`)
    (`SceneComponent.K2_SetRelativeRotation` (`self.SM_Stem`) (`KismetMathLibrary.FindLookAtRotation` (`KismetMathLibrary.MakeVector` _returnvalue_x _returnvalue_y) (`KismetMathLibrary.MakeVector` _returnvalue_x_2 _returnvalue_y_2)) false false)))

(event `One_Shot`
  ;[1 0.4941 0] One_Shot_Mechanic
  (`|SpawnActorFromClass` "/Game/Platformer/Blueprints/BP_Bullet.BP_Bullet_C" (`SceneComponent.GetSocketTransform` (`self.Firing_Point`) "None" "RTS_World") "Undefined" "MultiplyWithRoot" null null)
  ;[0.7608 0 0] Call One_Shot
  (`KismetSystemLibrary.Delay` (`self.Firing_Delay`))
  (`self.One_Shot`))

(event `Scattershot`
  (bind _returnvalue (`SceneComponent.GetSocketTransform` (`self.Firing_Point`) "None" "RTS_World"))
  ;[1 1 1] Scattershot
  (for _ (range 6)
    ;;[1 0.4941 0] Scattershot Mechanic
    (`|SpawnActorFromClass` "/Game/Platformer/Blueprints/BP_Bullet.BP_Bullet_C" (`KismetMathLibrary.MakeTransform` (.location _returnvalue) (`KismetMathLibrary.MakeRotator` (.roll (.rotation _returnvalue)) (.pitch (.rotation _returnvalue)) (+ (.yaw (.rotation _returnvalue)) (`KismetMathLibrary.RandomFloatInRange` -30.0 30.0)))) "Undefined" "MultiplyWithRoot" null null))
  ;;[0.7608 0 0] Call Scattershot
  (`KismetSystemLibrary.Delay` (`self.Firing_Delay`))
  (`self.Scattershot`))

(event `self.ReceiveBeginPlay`
  ;[0.003922 0.6157 0] Set Up: Firing Shot
  (if (`self.Use_Scattershot`)
    (`self.Scattershot`)
    (else
      (`self.One_Shot`))))

(fn `UserConstructionScript`)