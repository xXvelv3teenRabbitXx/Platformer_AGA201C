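; BP_Enemy_Chaser is a platformer enemy that chases the player and can be defeated by head bounces.
; Entering its Detection Zone starts a Tick-driven turn and chase; the reset on leaving is disconnected, so pursuit never stops.
; Overlapping the Hit Zone launches the player and removes enemy health, destroying it at zero.
; Capsule hits knock the player back using the enemy's scaled velocity and directly reduce player health.
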(event `self.ReceiveBeginPlay`
  ;[0.1294 0.4157 1] Get_Player_Reference
  (bind _asbp_third_person_character (cast `/Game/Platformer/Blueprints/BP_ThirdPersonCharacter` (`GameplayStatics.GetPlayerPawn` 0)))
  (set `self.Player_Reference` _asbp_third_person_character))

(event `self.Detection_Zone.OnComponentBeginOverlap`
  (params (OverlappedComponent :type "PrimitiveComponent Object Reference") (OtherActor :type "Actor Object Reference") (OtherComp :type "PrimitiveComponent Object Reference") (OtherBodyIndex :type Integer) (bFromSweep :type Boolean) (SweepResult :type "HitResult Structure (by ref)"))
  ;[0.1294 0.4157 1] Check: if_Detecting_Player
  (if (== OtherActor (`self.Player_Reference`))
    (set `self.Can_Detect_Player` true)))

(event `self.Detection_Zone.OnComponentEndOverlap`
  (params (OverlappedComponent :type "PrimitiveComponent Object Reference") (OtherActor :type "Actor Object Reference") (OtherComp :type "PrimitiveComponent Object Reference") (OtherBodyIndex :type Integer))
  ;[0.1294 0.4157 1] Check: if_Detecting_Player
)

(event `self.ReceiveTick`
  (params (DeltaSeconds :type "Float (single-precision)"))
  (bind (_returnvalue_x _returnvalue_y) (`KismetMathLibrary.BreakVector` (`self.K2_GetActorLocation`)))
  (bind (_returnvalue_x_2 _returnvalue_y_2) (`KismetMathLibrary.BreakVector` (`self.K2_GetActorLocation` (`self.Player_Reference`))))
  ;[0.1294 0.4157 1] if: Player_Detected
  (if (`self.Can_Detect_Player`)
    (`|ExecutionSequence`
      (:`then_0`
        ;[1 0.4941 0] Enemy_Look_At_Player
        (`self.K2_SetActorRotation` (`KismetMathLibrary.FindLookAtRotation` (`KismetMathLibrary.MakeVector` _returnvalue_x _returnvalue_y) (`KismetMathLibrary.MakeVector` _returnvalue_x_2 _returnvalue_y_2))))
      (:`then_1`
        ;[1 0.4941 0] Enemy_Chase_Player
        (`self.AddMovementInput` (`KismetMathLibrary.Normal` (- (`self.K2_GetActorLocation` (`self.Player_Reference`)) (`self.K2_GetActorLocation`))))))))

(event `self.Hit_Zone.OnComponentBeginOverlap`
  (params (OverlappedComponent :type "PrimitiveComponent Object Reference") (OtherActor :type "Actor Object Reference") (OtherComp :type "PrimitiveComponent Object Reference") (OtherBodyIndex :type Integer) (bFromSweep :type Boolean) (SweepResult :type "HitResult Structure (by ref)"))
  ;[0.1294 0.4157 1] Head_Bounce
  (if (== OtherActor (`self.Player_Reference`))
    (`|ExecutionSequence`
      (:`then_0`
        ;[1 0.4941 0] Launch_Player
        (`self.LaunchCharacter` (`self.Player_Reference`) (`self.Launch_Direction`) false false))
      (:`then_1`
        ;[1 0.4941 0] Pawn_Health and Destroy_Pawn
        (set `self.Chaser_Health` (- (`self.Chaser_Health`) 1))
        (if (<= (`self.Chaser_Health`) 0)
          (`self.K2_DestroyActor`))))))

(event `self.CapsuleComponent.OnComponentHit`
  (params (HitComponent :type "PrimitiveComponent Object Reference") (OtherActor :type "Actor Object Reference") (OtherComp :type "PrimitiveComponent Object Reference") (NormalImpulse :type "Vector Structure") (Hit :type "HitResult Structure (by ref)"))
  ;[1 0.4941 0] Knockback_Attack
  (if (== OtherActor (`self.Player_Reference`))
    (`self.LaunchCharacter` (`self.Player_Reference`) (* (`self.GetVelocity`) (`self.Knockback_Strength`)) false false)
    ;[1 0.4941 0] Damage_Player_Health
    (set `/Game/Platformer/Blueprints/BP_ThirdPersonCharacter.Player_Health` (- (`/Game/Platformer/Blueprints/BP_ThirdPersonCharacter.Player_Health` (`self.Player_Reference`)) (`self.Chaser_Damage`)) (`self.Player_Reference`))))

(fn `UserConstructionScript`)