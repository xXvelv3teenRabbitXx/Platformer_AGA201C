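; Platform that vanishes after the player has stood on it for a set lifetime, then reappears after a delay.
; Trigger-zone overlaps flag when the player pawn is on it, and Tick accumulates time while flagged, otherwise resetting it.
; At the limit it hides the actor and disables collision, then after a Delay restores visibility, collision and the transform saved at BeginPlay.
; Debug prints report overlaps and the running timer.
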(event `self.ReceiveBeginPlay`
  (bind (_returnvalue_location _returnvalue_rotation _returnvalue_scale) (`KismetMathLibrary.BreakTransform` (`self.GetTransform`)))
  ;[0.003922 0.6157 0] Set Starting Variables
  (set `self.Start_Location` _returnvalue_location)
  (set `self.Start_Rotation` _returnvalue_rotation)
  (set `self.Start_Scale` _returnvalue_scale))

(event `self.Platform_Trigger_Zone.OnComponentBeginOverlap`
  (params (OverlappedComponent :type "PrimitiveComponent Object Reference") (OtherActor :type "Actor Object Reference") (OtherComp :type "PrimitiveComponent Object Reference") (OtherBodyIndex :type Integer) (bFromSweep :type Boolean) (SweepResult :type "HitResult Structure (by ref)"))
  ;[1 0.4941 0] Collider Check
  (if (== OtherActor (`GameplayStatics.GetPlayerPawn` 0))
    (`|ExecutionSequence`
      (:`then_0`
        (`KismetSystemLibrary.PrintString` "Player is onPlatform"))
      (:`then_1`
        (set `self.Is_Player_On_Platform` true)))))

(event `self.Platform_Trigger_Zone.OnComponentEndOverlap`
  (params (OverlappedComponent :type "PrimitiveComponent Object Reference") (OtherActor :type "Actor Object Reference") (OtherComp :type "PrimitiveComponent Object Reference") (OtherBodyIndex :type Integer))
  ;[1 0.4941 0] Collider Check
  (if (== OtherActor (`GameplayStatics.GetPlayerPawn` 0))
    (`|ExecutionSequence`
      (:`then_0`
        (`KismetSystemLibrary.PrintString` "Player is offPlatform"))
      (:`then_1`
        (set `self.Is_Player_On_Platform` false)))))

(event `self.ReceiveTick`
  (params (DeltaSeconds :type "Float (single-precision)"))
  ;[0.003922 0.6157 0] Set Timer Platform
  (if (`self.Is_Player_On_Platform`)
    (bind _output_get (set `self.Time_On_Platform` (+ DeltaSeconds (`self.Time_On_Platform`))))
    (`|ExecutionSequence`
      (:`then_0`
        ;[0.003922 0.6157 0] If Timer has reached the Platform's Lifetime
        (if (>= (`self.Time_On_Platform`) (`self.Platform_Lifetime`))
          ;[0.003922 0.6157 0] Hide_and_Disable_Platform
          (`self.SetActorHiddenInGame` true)
          (`self.SetActorEnableCollision` false)
          (`KismetSystemLibrary.Delay` (`self.Time_Invisible`))
          (`self.Return_To_Start`)))
      (:`then_1`
        (`KismetSystemLibrary.PrintString` (`KismetStringLibrary.Conv_DoubleToString` _output_get))))
    (else
      (set `self.Time_On_Platform` 0.0))))

(event `Return_To_Start`
  ;[0.003922 0.6157 0] Return_To_Start
  (`SceneComponent.K2_SetWorldTransform` (`self.DefaultSceneRoot`) (`KismetMathLibrary.MakeTransform` (`self.Start_Location`) (`self.Start_Rotation`) (`self.Start_Scale`)) false true)
  (set `self.Time_On_Platform` 0.0)
  (`self.SetActorHiddenInGame` false)
  (`self.SetActorEnableCollision` true))

(fn `UserConstructionScript`)