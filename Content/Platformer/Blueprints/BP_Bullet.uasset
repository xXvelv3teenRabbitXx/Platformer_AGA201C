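; BP_Bullet is a projectile that damages the player on contact and destroys itself.
; Tick moves it by a local offset of normalized BulletDirection times BulletSpeed, without sweep or delta-time scaling.
; A Delay in Tick destroys it after BulletLifetime.
; Mesh overlap with the player pawn cached at BeginPlay subtracts BulletDamage directly from PlayerHealth and destroys the bullet, while other actors are ignored.
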(event `self.ReceiveBeginPlay`
  ;[0.1294 0.4157 1] Get_Player_Reference
  (bind _asbp_third_person_character (cast `/Game/Platformer/Blueprints/BP_ThirdPersonCharacter` (`GameplayStatics.GetPlayerPawn` 0)))
  (set `self.Player_Reference` _asbp_third_person_character))

(event `self.ReceiveTick`
  (params (DeltaSeconds :type "Float (single-precision)"))
  ;[0.1294 0.4157 1] Bullet_Movement
  (`self.K2_AddActorLocalOffset` (* (`KismetMathLibrary.Normal` (`self.Bullet_Direction`)) (`self.Bullet_Speed`)))
  ;[0.1294 0.4157 1] Destroy_Bullet
  (`KismetSystemLibrary.Delay` (`self.Bullet_Lifetime`))
  (`self.K2_DestroyActor`))

(event `self.SM_Bullet.OnComponentBeginOverlap`
  (params (OverlappedComponent :type "PrimitiveComponent Object Reference") (OtherActor :type "Actor Object Reference") (OtherComp :type "PrimitiveComponent Object Reference") (OtherBodyIndex :type Integer) (bFromSweep :type Boolean) (SweepResult :type "HitResult Structure (by ref)"))
  ;[1 0.4941 0] Damage_Player_Health + Destroy_Bullet
  (if (== OtherActor (`self.Player_Reference`))
    (set `/Game/Platformer/Blueprints/BP_ThirdPersonCharacter.Player_Health` (- (`/Game/Platformer/Blueprints/BP_ThirdPersonCharacter.Player_Health` (`self.Player_Reference`)) (`self.Bullet_Damage`)) (`self.Player_Reference`))
    (`self.K2_DestroyActor`)))

(fn `UserConstructionScript`)